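; Player controller for the Snake game that owns the on-screen widget and relays game events to the game mode.
; It shows the HUD on begin play, swapping it for game over, victory or a fresh HUD on death, win or restart.
; Picking fruit increments the game mode's fruit count and refreshes the HUD, while death also tells the game mode to stop the game.
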(event `self.ReceiveBeginPlay`
  (bind _returnvalue (`|CreateWidget` "/Game/SnakeBP/UI/WBP_UserIntrerface.WBP_UserIntrerface_C"))
  (bind _output_get (set `self.UserWidget` _returnvalue))
  (`UserWidget.AddToViewport` _output_get 0))

(event `PickFruit`
  (bind _asbp_gmsnake (cast `/Game/SnakeBP/Blueprints/BP_GMSnake` (`GameplayStatics.GetGameMode`)))
  (`/Game/SnakeBP/Blueprints/BP_GMSnake.AddFruitCount` _asbp_gmsnake)
  (bind _userwidget (`self.UserWidget`)
    (:`then`
      (bind _aswbp_user_intrerface (cast `/Game/SnakeBP/UI/WBP_UserIntrerface` _userwidget))
      (`/Game/SnakeBP/UI/WBP_UserIntrerface.UpdateData` _aswbp_user_intrerface))
    (:`else`)))

(event `Dead`
  (`Widget.RemoveFromParent` (`self.UserWidget`))
  (bind _returnvalue (`|CreateWidget` "/Game/SnakeBP/UI/WBP_GameOver.WBP_GameOver_C"))
  (bind _output_get (set `self.UserWidget` _returnvalue))
  (`UserWidget.AddToViewport` _output_get 0)
  (bind _asbp_gmsnake (cast `/Game/SnakeBP/Blueprints/BP_GMSnake` (`GameplayStatics.GetGameMode`)))
  (`/Game/SnakeBP/Blueprints/BP_GMSnake.StopGame` _asbp_gmsnake))

(event `RestartGame`
  (`Widget.RemoveFromParent` (`self.UserWidget`))
  (bind _returnvalue (`|CreateWidget` "/Game/SnakeBP/UI/WBP_UserIntrerface.WBP_UserIntrerface_C"))
  (bind _output_get (set `self.UserWidget` _returnvalue))
  (`UserWidget.AddToViewport` _output_get 0))

(event `UI_Victory`
  (`Widget.RemoveFromParent` (`self.UserWidget`))
  (bind _returnvalue (`|CreateWidget` "/Game/SnakeBP/UI/WBP_Victory.WBP_Victory_C"))
  (bind _output_get (set `self.UserWidget` _returnvalue))
  (`UserWidget.AddToViewport` _output_get 0))

(fn `UserConstructionScript`)