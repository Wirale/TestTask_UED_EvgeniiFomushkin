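; Game mode for the Snake game that manages pickups, fruit score, victory and restarts.
; It keeps one fruit, spawned on BeginPlay and replaced via SpawnFruit, and a random-type CoreItem respawned on a looping timer, both at random points in the play area.
; AddFruitCount triggers the controller's victory UI and pauses at the target count.
; StartGame unpauses, respawns and possesses a new snake, and resets the count and controller.
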(event `self.ReceiveBeginPlay`
  (`self.SpawnFruit`)
  (`KismetSystemLibrary.K2_SetTimer` null "SpawnItem" 10.0 true))

(event `SpawnItem`
  (bind _item (`self.Item`)
    (:`then`
      (`self.K2_DestroyActor` _item))
    (:`else`
      _))
  (bind _returnvalue (`|SpawnActorFromClass` "/Game/ItemBP/CoreItem.CoreItem_C" (`KismetMathLibrary.MakeTransform` (`KismetMathLibrary.RandomPointInBoundingBox` (0.0 0.0 0.0) (1000.0 1000.0 0.0))) "AlwaysSpawn" "OverrideRootScale" null (cast `/Game/ItemBP/TypeItem` (`KismetMathLibrary.Conv_IntToByte` (`KismetMathLibrary.RandomIntegerInRange` 1 3))) null))
  (set `self.Item` _returnvalue))

(event `StopGame`
  (`GameplayStatics.SetGamePaused` true))

(event `StartGame`
  (bind _returnvalue (`GameplayStatics.GetPlayerController` 0))
  (`GameplayStatics.SetGamePaused` false)
  (`self.K2_DestroyActor` (`GameplayStatics.GetPlayerPawn` 0))
  (bind _returnvalue_2 (`|SpawnActorFromClass` "/Game/SnakeBP/Blueprints/BP_Snake.BP_Snake_C" (`self.GetTransform` (`self.K2_FindPlayerStart` (`GameplayStatics.GetPlayerController` 0))) "AlwaysSpawn" "OverrideRootScale" null null))
  (`Controller.Possess` _returnvalue _returnvalue_2)
  (set `self.CurrentCountFruit` 0)
  (bind _asbp_snake_controller (cast `/Game/SnakeBP/Blueprints/BP_SnakeController` _returnvalue))
  (`/Game/SnakeBP/Blueprints/BP_SnakeController.RestartGame` _asbp_snake_controller))

(fn `AddFruitCount`
  (`/Engine/EditorBlueprintResources/StandardMacros.IncrementInt` (`self.CurrentCountFruit`)
    (:`  `
      (if (== (`self.CurrentCountFruit`) (`self.MaxCountFruit`))
        (bind _asbp_snake_controller (cast `/Game/SnakeBP/Blueprints/BP_SnakeController` (`GameplayStatics.GetPlayerController` 0)))
        (`/Game/SnakeBP/Blueprints/BP_SnakeController.UI_Victory` _asbp_snake_controller)
        (`self.StopGame`)))))

(fn `GetCurrentCountFruit`
  (returns (CurrentCountFruit :type Integer))
  (return (`self.CurrentCountFruit`)))

(fn `GetMaxCountFruit`
  (returns (MaxCountFruit :type Integer))
  (return (`self.MaxCountFruit`)))

(fn `SpawnFruit`
  (bind _fruit (`self.Fruit`)
    (:`then`
      (`self.K2_DestroyActor` _fruit))
    (:`else`
      _))
  (bind _returnvalue (`|SpawnActorFromClass` "/Game/ItemBP/CoreItem.CoreItem_C" (`KismetMathLibrary.MakeTransform` (`KismetMathLibrary.RandomPointInBoundingBox` (0.0 0.0 0.0) (1000.0 1000.0 0.0))) "AlwaysSpawn" "OverrideRootScale" null "NewEnumerator0" null))
  (set `self.Fruit` _returnvalue))

(fn `UserConstructionScript`)