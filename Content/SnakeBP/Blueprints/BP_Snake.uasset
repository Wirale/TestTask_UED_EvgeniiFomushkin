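; BP_Snake is the player-controlled pawn of a Snake game, steered with WASD in 100-unit steps without direct reversal.
; A looping timer runs MoveSnake, which shifts instanced-mesh tail segments toward the head, then sphere-traces the next position before moving.
; Items grow and speed up the snake, temporarily change the timer rate, or kill it.
; Hitting a snake or blocking volume also calls Dead on the controller.
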(event `self.ReceiveBeginPlay`
  (bind _returnvalue (`KismetSystemLibrary.K2_SetTimer` null "MoveSnake" (`self.TimeMove`) true))
  (set `self.TimerSpeedGame` _returnvalue)
  (`InstancedStaticMeshComponent.AddInstance` (`self.HierarchicalInstancedStaticMesh`) (`KismetMathLibrary.MakeTransform` (* (`SceneComponent.GetForwardVector` (`self.HeadSnake`)) -100.0)))
  (for _index (range 3 (+ (`self.StartCount`) 1))
    (`InstancedStaticMeshComponent.AddInstance` (`self.HierarchicalInstancedStaticMesh`) (`KismetMathLibrary.MakeTransform` (+ (.location (`InstancedStaticMeshComponent.GetInstanceTransform` (`self.HierarchicalInstancedStaticMesh`) (- _index 1) false)) (* (`SceneComponent.GetForwardVector` (`self.HeadSnake`)) -100.0))))))

(event `MoveSnake`
  (bind _headsnake (`self.HeadSnake`))
  (bind _returnvalue (+ (`SceneComponent.K2_GetComponentLocation` (`self.HeadSnake`)) (`self.MoveVector`)))
  (`self.RelocationTail`)
  (bind (_outhit _returnvalue_2) (`KismetSystemLibrary.SphereTraceSingleForObjects` :`Start` _returnvalue :`End` _returnvalue :`Radius` 30.0 :`ObjectTypes` (`|MakeArray` "ObjectTypeQuery1" :!type "EObjectTypeQuery Enum") :`bIgnoreSelf` false :`DrawTime` 1.0))
  (if _returnvalue_2
    (bind (_bblockinghit _binitialoverlap _time _distance _location _impactpoint _normal _impactnormal _physmat _hitactor) (`GameplayStatics.BreakHitResult` _outhit))
    (bind _ascore_item (cast `/Game/ItemBP/CoreItem` _hitactor)
      (:`then`
        (`self.SelectAction` (`/Game/ItemBP/CoreItem.GetTypeItem` _ascore_item))
        (`/Engine/EditorBlueprintResources/StandardMacros.IsValid` _hitactor
          (:`Is Valid`
            (`self.K2_DestroyActor` _hitactor))
          (:`Is Not Valid`
            _))
        (`SceneComponent.K2_SetWorldLocation` _headsnake (+ (`SceneComponent.K2_GetComponentLocation` _headsnake) (`self.MoveVector`)) false true :!label _label))
      (:`CastFailed`
        (cast `/Game/SnakeBP/Blueprints/BP_Snake` _hitactor
          (:`then`
            _)
          (:`CastFailed`
            (cast `BlockingVolume` _hitactor
              (:`then`
                _)
              (:`CastFailed`
                (goto _label)))))
        (bind _asbp_snake_controller (cast `/Game/SnakeBP/Blueprints/BP_SnakeController` (`self.GetController`)))
        (`/Game/SnakeBP/Blueprints/BP_SnakeController.Dead` _asbp_snake_controller)))
    (else
      (goto _label))))

(event `DefaultSpeed`
  (`KismetSystemLibrary.K2_ClearAndInvalidateTimerHandle` (`self.TimerSpeedGame`))
  (bind _returnvalue (`KismetSystemLibrary.K2_SetTimer` null "MoveSnake" (`self.TimeMove`) true))
  (set `self.TimerSpeedGame` _returnvalue))

(event `Key|W`
  (params (Key :type "Key Structure"))
  (:`Pressed`
    (if (not (== (`self.LastKey`) 1))
      (set `self.MoveVector` (100.0 0.0 0.0))
      (set `self.LastKey` 0))))

(event `Key|S`
  (params (Key :type "Key Structure"))
  (:`Pressed`
    (if (not (== (`self.LastKey`) 0))
      (set `self.MoveVector` (-100.0 0.0 0.0))
      (set `self.LastKey` 1))))

(event `Key|D`
  (params (Key :type "Key Structure"))
  (:`Pressed`
    (if (not (== (`self.LastKey`) 3))
      (set `self.MoveVector` (0.0 100.0 0.0))
      (set `self.LastKey` 2))))

(event `Key|A`
  (params (Key :type "Key Structure"))
  (:`Pressed`
    (if (not (== (`self.LastKey`) 2))
      (set `self.MoveVector` (0.0 -100.0 0.0))
      (set `self.LastKey` 3))))

(fn `AddTail`
  (bind _hierarchicalinstancedstaticmesh (`self.HierarchicalInstancedStaticMesh`))
  (bind _returnvalue (- (`self.TimeMove`) 0.05))
  (`InstancedStaticMeshComponent.AddInstance` _hierarchicalinstancedstaticmesh (`InstancedStaticMeshComponent.GetInstanceTransform` _hierarchicalinstancedstaticmesh (- (`InstancedStaticMeshComponent.GetInstanceCount` _hierarchicalinstancedstaticmesh) 1) false))
  (if (not (< _returnvalue 0.0))
    (bind _output_get (set `self.TimeMove` _returnvalue))
    (`self.ControlSpeed` _output_get)))

(fn `ControlSpeed`
  (params (Time :type "Float (double-precision)"))
  (`KismetSystemLibrary.K2_ClearAndInvalidateTimerHandle` (`self.TimerSpeedGame`))
  (bind _returnvalue (`KismetSystemLibrary.K2_SetTimer` null "MoveSnake" Time true))
  (set `self.TimerSpeedGame` _returnvalue))

(fn `RelocationTail`
  (locals (LocalIndex :type Integer) (LocalVectorOne :type "Vector Structure") (LocalVectorTwo :type "Vector Structure"))
  (set `local.LocalIndex` (`InstancedStaticMeshComponent.GetInstanceCount` (`self.HierarchicalInstancedStaticMesh`)))
  (set `local.LocalVectorOne` (`SceneComponent.K2_GetComponentLocation` (`self.HeadSnake`)))
  (for _index (range (+ (`local.LocalIndex`) 1))
    (set `local.LocalVectorTwo` (.location (`InstancedStaticMeshComponent.GetInstanceTransform` (`self.HierarchicalInstancedStaticMesh`) _index false)))
    (`InstancedStaticMeshComponent.UpdateInstanceTransform` (`self.HierarchicalInstancedStaticMesh`) _index (`KismetMathLibrary.MakeTransform` (`local.LocalVectorOne`)) false false true)
    (set `local.LocalVectorOne` (`local.LocalVectorTwo`))))

(fn `SelectAction`
  (params (Selection :type "/Game/ItemBP/TypeItem Enum" :default "NewEnumerator0"))
  (bind _timemove (`self.TimeMove`))
  (switch `/Game/ItemBP/TypeItem` Selection
    (:`NewEnumerator0`
      (bind _asbp_snake_controller (cast `/Game/SnakeBP/Blueprints/BP_SnakeController` (`self.GetController`)))
      (`/Game/SnakeBP/Blueprints/BP_SnakeController.PickFruit` _asbp_snake_controller)
      (bind _asbp_gmsnake (cast `/Game/SnakeBP/Blueprints/BP_GMSnake` (`GameplayStatics.GetGameMode`)))
      (`/Game/SnakeBP/Blueprints/BP_GMSnake.SpawnFruit` _asbp_gmsnake)
      (`self.AddTail`))
    (:`NewEnumerator1`
      (`self.ControlSpeed` (/ _timemove 2.0))
      (`KismetSystemLibrary.K2_SetTimer` null "DefaultSpeed" 6.0 :!label _label))
    (:`NewEnumerator2`
      (`self.ControlSpeed` (* _timemove 2.0))
      (goto _label))
    (:`NewEnumerator3`
      (bind _asbp_snake_controller_2 (cast `/Game/SnakeBP/Blueprints/BP_SnakeController` (`self.GetController`)))
      (`/Game/SnakeBP/Blueprints/BP_SnakeController.Dead` _asbp_snake_controller_2))))

(fn `UserConstructionScript`)